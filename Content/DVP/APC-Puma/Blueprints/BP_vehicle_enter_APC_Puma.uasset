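; Handles the player entering the APC Puma vehicle, with an on-screen enter prompt.
; Display_text adds the enter widget to the viewport when NearVehicle is set, and removes it otherwise.
; Enter_vehicle, gated by UseVehicle and NearVehicle, hands the player character to the vehicle pawn and possesses it.
; It then hides the character, disables its collision, hides the vehicle's third-person health widget and removes the prompt.
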(event Custom|Display_text
  ;[1 1 1] Display enter text
  (if (Variables|Default|GetbNear_vehicle_?)
    (bind _returnvalue (UserInterface|CreateWidget "/Game/DVP/APC-Puma/UI/UMG_APC_Puma_Vehicle_enter.UMG_APC_Puma_Vehicle_enter_C" (Game|GetPlayerController 0)))
    (UserInterface|Viewport|AddtoViewport _returnvalue 0)
    (else
      (Utilities|IsValid _returnvalue
        (:Is%20Valid
          (Widget|RemovefromParent _returnvalue))))))

(event Custom|Enter_vehicle
  (bind _vehicle_p (Variables|Default|GetVehicle_P))
  ;[1 1 1] Posses vehicle
  (if (and (Variables|Default|GetbUse_vehicle) (Variables|Default|GetbNear_vehicle_?))
    (Variables|/Game/DVP/APC-Puma/Blueprints/BP_APC_Puma.BP_APC_Puma_C|SetUse%20APC%20Puma _vehicle_p true)
    (bind _output_get (Variables|/Game/DVP/APC-Puma/Blueprints/BP_APC_Puma.BP_APC_Puma_C|SetCharacter _vehicle_p (Game|GetPlayerCharacter 0)))
    (Pawn|Possess (Game|GetPlayerController 0) _vehicle_p)
    (Rendering|SetActorHiddenInGame _output_get true)
    (Collision|SetActorEnableCollision _output_get false)
    (Rendering|SetVisibility (Variables|/Game/DVP/APC-Puma/Blueprints/BP_APC_Puma.BP_APC_Puma_C|GetWidget_3P_Health _vehicle_p) false false)
    ;[1 1 1] Display enter text
    (Widget|RemovefromParent (stale Custom|Display_text _returnvalue))))