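; BP_AssaultClass is the Assault character class, with a class skill that trades health for a short speed burst.
; Using the skill calls a Server event that raises the run speed modifier and damages the character itself, then, after a delay, ServerResetRun restores the default modifier.
; The construction script selects the AK-47 as primary weapon and a test secondary weapon to spawn.
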(event Custom|Server
  (bind _self self)
  ;[0.8079 1 0.4961] Class Skill
  (Variables|Default|SetRunSpeedModifier 2.5)
  (Game|Damage|ApplyDamage _self 1e+01 0 _self))

(event Custom|ServerResetRun
  ;[0.8079 1 0.4961] Class Skill
  (Variables|Default|SetRunSpeedModifier (Variables|Default|GetDefaultRunSpeedModdifier)))

(event EventBeginPlay
  (|CallParentFunction))

(event Collision|EventActorBeginOverlap
  (params (OtherActor :type Actor%20Object%20Reference)))

(event EventTick
  (params (DeltaSeconds :type Float%20%28single-precision%29))
  (|CallParentFunction DeltaSeconds) ; This node is disabled and will not be called.\nDrag off pins to build functionality.
)

(event EventUseClassSkill
  ;[0.8079 1 0.4961] Class Skill
  (CallFunction|Server)
  (Utilities|FlowControl|Delay 2.0)
  (CallFunction|ServerResetRun))

(fn ConstructionScript
  (|CallParentFunction)
  (Variables|Default|SetPrimaryWeaponToSpawn "/Game/FPS/Blueprints/Weapons/BP_AssaultWeapon_Ak47.BP_AssaultWeapon_Ak47_C")
  (Variables|Default|SetSecondaryWeaponToSpawn "/Game/FPS/Blueprints/Weapons/BP_SecondaryWeaponTest.BP_SecondaryWeaponTest_C"))