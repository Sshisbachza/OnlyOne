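; Handles the player's entry into the LSV Rhino vehicle, with an on-screen enter prompt.
; Display_text shows the prompt widget when the player is near the vehicle's left or right door, and removes it otherwise.
; Enter_vehicle opens the nearby door, possesses the vehicle, hides the character and disables its collision.
; On entry it also stores the character on the vehicle, hides the vehicle's health widget and clears the prompt.
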(event Custom|Display_text
  (bind _vehicle_p (Variables|Default|GetVehicle_P))
  ;[1 1 1] Display enter text
  (if (and (Variables|Default|GetbNear_vehicle_?) (or (Variables|/Game/DVP/LSV-Rhino/Blueprints/BP_LSV_Rhino.BP_LSV_Rhino_C|GetbNear_LSV_Leftt_Door_? _vehicle_p) (Variables|/Game/DVP/LSV-Rhino/Blueprints/BP_LSV_Rhino.BP_LSV_Rhino_C|GetbNear_LSV_Right_Door_? _vehicle_p)))
    (bind _returnvalue (UserInterface|CreateWidget "/Game/DVP/LSV-Rhino/UI/UMG_LSV_Vehicle_enter.UMG_LSV_Vehicle_enter_C" (Game|GetPlayerController 0)))
    (UserInterface|Viewport|AddtoViewport _returnvalue 0)
    (elif (Utilities|IsValid _returnvalue)
      (Widget|RemovefromParent _returnvalue))))

(event Custom|Enter_vehicle
  (bind _vehicle_p (Variables|Default|GetVehicle_P))
  (bind _vehicle_p_2 (Variables|Default|GetVehicle_P))
  ;[1 1 1] Posses vehicle
  (if (and (Variables|Default|GetbUse_vehicle) (Variables|Default|GetbNear_vehicle_?))
    (Utilities|FlowControl|Sequence
      (:then_0
        (if (Variables|/Game/DVP/LSV-Rhino/Blueprints/BP_LSV_Rhino.BP_LSV_Rhino_C|GetbNear_LSV_Leftt_Door_? _vehicle_p_2)
          (Default|OpenLeftDoor _vehicle_p_2)
          (Variables|/Game/DVP/LSV-Rhino/Blueprints/BP_LSV_Rhino.BP_LSV_Rhino_C|SetUse_LSV _vehicle_p true :!label _label)
          (bind _output_get (Variables|/Game/DVP/LSV-Rhino/Blueprints/BP_LSV_Rhino.BP_LSV_Rhino_C|SetCharacter _vehicle_p (Game|GetPlayerCharacter 0)))
          (Pawn|Possess (Game|GetPlayerController 0) _vehicle_p)
          (Rendering|SetActorHiddenInGame _output_get true)
          (Collision|SetActorEnableCollision _output_get false)
          (Rendering|SetVisibility (Variables|/Game/DVP/LSV-Rhino/Blueprints/BP_LSV_Rhino.BP_LSV_Rhino_C|GetWidget_3P_Health _vehicle_p) false false)
          ;[1 1 1] Display enter text
          (if (Utilities|IsValid (stale Custom|Display_text _returnvalue))
            (Widget|RemovefromParent (stale Custom|Display_text _returnvalue)))))
      (:then_1
        (if (Variables|/Game/DVP/LSV-Rhino/Blueprints/BP_LSV_Rhino.BP_LSV_Rhino_C|GetbNear_LSV_Right_Door_? _vehicle_p_2)
          (Default|OpenRightDoor _vehicle_p_2)
          (goto _label))))))