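; FPS player state that keeps a player's kill and death score.
; Events reset both counters, add a death, or register a kill, with team kills subtracting one from the kill count.
; The construction script stores the result of GetPlayerName in a Name variable.
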(event Custom|AddKill
  (params (TeamKill :type Boolean))
  ;[1 1 1] AddKill
  (Variables|Default|SetKills (select TeamKill (- (Variables|Default|GetKills) 1) (+ (Variables|Default|GetKills) 1))))

(event Custom|ResetScore
  ;[1 1 1] ResetScore
  (Variables|Default|SetKills 0)
  (Variables|Default|SetDeaths 0))

(event Custom|AddDeath
  ;[1 1 1] AddDeath
  (Variables|Default|SetDeaths (+ (Variables|Default|GetDeaths) 1)))

(fn ConstructionScript
  (Variables|Default|SetName (PlayerState|GetPlayerName)))