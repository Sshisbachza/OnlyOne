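; Test character class for the FPS game, with a mine-laying class skill and its own weapon loadout.
; UseClassSkill spends one of the remaining Traps, then line-traces forward and downward from the character to pick a location.
; ServerSpawnMine spawns BP_Mine at that location, without a hit check, with the character as instigator.
; The construction script assigns the support weapon as primary and a test weapon as secondary.
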(event Custom|ServerSpawnMine
  (params (NewParam :type Transform))
  ;[0.6685 0.7443 1] Class Skill
  (Game|SpawnActorfromClass "/Game/FPS/Blueprints/Misc/Mine/BP_Mine.BP_Mine_C" NewParam "Undefined" 0 self))

(event EventBeginPlay
  (|CallParentFunction) ; This node is disabled and will not be called.\nDrag off pins to build functionality.
)

(event Collision|EventActorBeginOverlap
  (params (OtherActor :type Actor%20Object%20Reference)))

(event EventTick
  (params (DeltaSeconds :type Float%20%28single-precision%29)))

(event EventUseClassSkill
  (bind _returnvalue (Transformation|GetActorLocation))
  ;[0.6685 0.7443 1] Class Skill
  (if (!= (Variables|Default|GetTraps) 0)
    (bind _result (Math|Integer|DecrementInt (Variables|Default|GetTraps))
      (:%20%20
        (Variables|Default|SetTraps _result)
        (bind _outhit (Collision|LineTraceByChannel _returnvalue (+ _returnvalue (+ (* (Transformation|GetActorForwardVector) 1e+03) (* (Transformation|GetActorUpVector) -5e+02))) "TraceTypeQuery1" false 0 "None"))
        (CallFunction|ServerSpawnMine (Math|Conversions|ToTransform(Vector) (.location _outhit)))))))

(fn ConstructionScript
  (|CallParentFunction)
  (Variables|Default|SetPrimaryWeaponToSpawn "/Game/FPS/Blueprints/Weapons/BP_SupportWeapon.BP_SupportWeapon_C")
  (Variables|Default|SetSecondaryWeaponToSpawn "/Game/FPS/Blueprints/Weapons/BP_SecondaryWeaponTest.BP_SecondaryWeaponTest_C"))