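; Rocket projectile for the AH Sparrow that damages whatever it hits and ignores its instigator while moving.
; Every hit applies damage, then a one-time sequence fires a radial force impulse with impact particles and sound.
; It then destroys its components and, after a short delay, the actor.
; An unconnected class check could restrict damage to BP_AH_Sparrow targets.
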(event EventBeginPlay
  ;[1 1 1] Rocket projectile
  (Collision|IgnoreActorwhenMoving (Variables|MyProjectile|GetCollisionComponent) (Game|GetInstigator) true))

(event Collision|EventHit
  (params (MyComp :type Primitive%20Component%20Object%20Reference) (Other :type Actor%20Object%20Reference) (OtherComp :type Primitive%20Component%20Object%20Reference) (bSelfMoved :type Boolean) (HitLocation :type Vector) (HitNormal :type Vector :default "0, 0, 0") (NormalImpulse :type Vector :default "0, 0, 0") (Hit :type Hit%20Result%20Structure%20%28by%20ref%29))
  (bind _tracestart (Collision|BreakHitResult Hit))
  (bind _staticmesh (Variables|Default|GetStaticMesh))
  (bind (_x _y) (Math|Vector|BreakVector _tracestart))
  (bind _returnvalue (Transformation|GetWorldLocation _staticmesh))
  ;[1 1 1] Rocket projectile
  (Game|Damage|ApplyDamage Other (Variables|Default|GetRocket_damage_caused) 0 0) ; How much damage is delt by Rocket
  (Utilities|FlowControl|DoOnce false
    (:Completed
      (Class|RadialForceComponent|FireImpulse (Variables|MyProjectile|GetRadialForce1))
      (Effects|SpawnEmitteratLocation "/Game/DVP/APC-Puma/Particles/PS_Impact_APC_main_gun.PS_Impact_APC_main_gun" _returnvalue (Math|Rotator|MakeRotator _x _y 0.0))
      (Audio|PlaySoundatLocation "/Game/DVP/APC-Puma/Sounds/Cues/SC_APC_Main_Gun_impact.SC_APC_Main_Gun_impact" _returnvalue "0, 0, 0" 1.0 1.0 0.0 "/Game/DVP/AH-Sparrow/Sounds/Rocket_att.Rocket_att")
      (Utilities|FlowControl|Delay 0.01)
      (Components|DestroyComponent (Variables|Default|GetStaticMesh))
      (Utilities|FlowControl|Delay 1.0)
      (Actor|DestroyActor))))

(fn ConstructionScript)