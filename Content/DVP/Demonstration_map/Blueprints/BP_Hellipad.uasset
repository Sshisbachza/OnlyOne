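; Helipad actor for the demonstration map that animates the brightness of its lights from BeginPlay.
; A single timeline's Emissive track, scaled, drives the Emissive_power material parameter on four static meshes and the intensity of four point lights together.
; The construction script is empty, and its leftover red lightbulb dynamic material setup is disconnected, so the meshes' material parameters are set directly.
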(event EventBeginPlay
  (bind _emissive (Timeline|Timeline_0 PlayFromStart)
    (:Update
      (Utilities|FlowControl|Sequence
        (:then_0
          (Rendering|Material|SetScalarParameterValueonMaterials (Variables|Default|GetStaticMesh2) "Emissive_power" (* _emissive 5.0)))
        (:then_1
          (Rendering|Material|SetScalarParameterValueonMaterials (Variables|Default|GetStaticMesh1) "Emissive_power" (* _emissive 5.0)))
        (:then_2
          (Rendering|Material|SetScalarParameterValueonMaterials (Variables|Default|GetStaticMesh4) "Emissive_power" (* _emissive 5.0)))
        (:then_3
          (Rendering|Material|SetScalarParameterValueonMaterials (Variables|Default|GetStaticMesh6) "Emissive_power" (* _emissive 5.0)))
        (:then_4
          (Rendering|Components|Light|SetIntensity (Variables|Default|GetPointLight1) (* _emissive 5e+01)))))))

(fn ConstructionScript)