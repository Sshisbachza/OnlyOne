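; BP_VehicleSpawn is a spawner actor that keeps a BP_BaseVehicle present at its Arrow component's transform.
; Shortly after BeginPlay it spawns a vehicle with authority only and stores the reference.
; A looping timer periodically checks that reference and spawns a replacement once the vehicle is no longer valid.
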(event Custom|RespawnVehicle
  (Utilities|IsValid (Variables|Default|GetVehicle)
    (:Is%20Not%20Valid
      (CallFunction|SpawnVehicle))))

(event Custom|SpawnVehicle
  ;[1 1 1] Spawn vehicle
  (Networking|SwitchHasAuthority
    (:Authority
      (bind _returnvalue (Game|SpawnActorfromClass "/Game/FPS/Blueprints/VehicleAdvBP/BP_BaseVehicle.BP_BaseVehicle_C" (Transformation|GetWorldTransform (Variables|Default|GetArrow)) "Undefined" 0 0))
      (Variables|Default|SetVehicle _returnvalue))))

(event EventBeginPlay
  (Utilities|FlowControl|Delay 1.0)
  (CallFunction|SpawnVehicle)
  (Utilities|Time|SetTimerbyEvent (delegate Custom|RespawnVehicle) 5.0 true))

(fn ConstructionScript)