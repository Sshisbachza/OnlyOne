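; BP_MedicClass is the medic character class for the FPS, assigning the medic primary weapon and a test secondary weapon in its construction script.
; Its class skill spawns a BP_MedicBot high above the character, passing it the owning pawn and the team read from player controller 0.
; A BotDeployed flag blocks further spawns until ResetBot clears it after a short delay.
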(event Custom|SpawnMedicBot
  (params (NewParam :type BP%20Base%20Character%20Object%20Reference) (bTeam :type Boolean))
  (bind _self self)
  (bind _returnvalue (Transformation|GetActorLocation _self))
  ;[1 1 1] Spawn Medic Bot
  (if (not (Variables|Default|GetbBotDeployed))
    (bind _returnvalue_2 (Game|SpawnActorfromClass "/Game/FPS/Blueprints/AI_Pawns/MedicBot/BP_MedicBot.BP_MedicBot_C" (Math|Transform|MakeTransform (Math|Vector|MakeVector (.x _returnvalue) (.y _returnvalue) (+ (.z _returnvalue) 1e+03)) (Transformation|GetActorRotation _self) "1,1,1") "Undefined" NewParam 0))
    (Variables|/Game/FPS/Blueprints/AI_Pawns/MedicBot/BP_MedicBot.BP_MedicBot_C|SetbBotTeam _returnvalue_2 bTeam)
    (Variables|/Game/FPS/Blueprints/AI_Pawns/MedicBot/BP_MedicBot.BP_MedicBot_C|SetOwnerPawn _returnvalue_2 self)
    (Variables|Default|SetbBotDeployed true)))

(event Custom|ResetBot
  ;[1 1 1] Bot Coldown
  (Utilities|FlowControl|Delay 2.0)
  (Variables|Default|SetbBotDeployed false))

(event EventBeginPlay
  (|CallParentFunction))

(event EventUseClassSkill
  ;[1 1 1] Medic Skill
  (CallFunction|SpawnMedicBot self (Variables|/Game/FPS/Blueprints/PlayerController/BaseCharacterPC.BaseCharacterPC_C|GetTeam (.AsBase%20Character%20PC (Utilities|Casting|CastToBaseCharacterPC (Game|GetPlayerController 0))))))

(event EventTick
  (params (DeltaSeconds :type Float%20%28single-precision%29))
  (|CallParentFunction DeltaSeconds))

(fn ConstructionScript
  (|CallParentFunction)
  (Variables|Default|SetPrimaryWeaponToSpawn "/Game/FPS/Blueprints/Weapons/BP_MedicWeapon.BP_MedicWeapon_C")
  (Variables|Default|SetSecondaryWeaponToSpawn "/Game/FPS/Blueprints/Weapons/BP_SecondaryWeaponTest.BP_SecondaryWeaponTest_C"))