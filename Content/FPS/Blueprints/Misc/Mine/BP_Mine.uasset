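; BP_Mine is a proximity mine that explodes when a BP_BaseCharacter overlaps its sphere on the server, or when it takes damage.
; Both triggers share one path that applies full radial damage from slightly above the mine, multicasts explosion particles and sound, then destroys the actor after a brief delay.
; A Destroyed flag limits the damage trigger to one detonation, but the overlap trigger does not check it.
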(event OnComponentBeginOverlap(Sphere)
  (params (OverlappedComponent :type Primitive%20Component%20Object%20Reference) (OtherActor :type Actor%20Object%20Reference) (OtherComp :type Primitive%20Component%20Object%20Reference) (OtherBodyIndex :type Integer) (bFromSweep :type Boolean) (SweepResult :type Hit%20Result%20Structure%20%28by%20ref%29))
  (bind _self self)
  (bind _returnvalue (Transformation|GetActorLocation _self))
  (bind (_x _y _z) (Math|Vector|BreakVector _returnvalue))
  ;[1 1 1] On Overlap
  (Networking|SwitchHasAuthority
    (:Authority
      (Utilities|Casting|CastToBP_BaseCharacter OtherActor)
      (Game|Damage|ApplyRadialDamage 1.5e+02 (Math|Vector|MakeVector _x _y (+ _z 3e+01)) 5e+02 0 (Utilities|Array|MakeArray self) (stale Game|Damage|EventAnyDamage DamageCauser) 0 true "ECC_Visibility")
      (CallFunction|PlayEffectsMulti)
      (Utilities|FlowControl|Delay 0.1)
      (Actor|DestroyActor))))

(event Custom|PlayEffectsMulti
  (bind _self self)
  (bind _returnvalue (Transformation|GetActorLocation _self))
  ;[1 1 1] PlayEffects Multicast
  (Effects|SpawnEmitteratLocation "/Game/FPS/Effects/WeaponEffects/Explosion/P_Explosion.P_Explosion" _returnvalue "0, 0, 0" "3.000000,3.000000,3.000000")
  (Audio|PlaySoundatLocation "/Game/FPS/MusicSound/Sounds/Explosions/Explosion_03.Explosion_03" _returnvalue "0, 0, 0" 1.0 1.0 0.0 "/Game/FPS/MusicSound/WeaponAttenuation.WeaponAttenuation" 0 0))

(event Game|Damage|EventAnyDamage
  (params (Damage :type Float%20%28single-precision%29) (DamageType :type Damage%20Type%20Object%20Reference) (InstigatedBy :type Controller%20Object%20Reference) (DamageCauser :type Actor%20Object%20Reference))
  (bind _self self)
  (bind _returnvalue (Transformation|GetActorLocation _self))
  (bind (_x _y _z) (Math|Vector|BreakVector _returnvalue))
  ;[1 1 1] On Overlap
  (if (not (Variables|Default|GetbDestroyed))
    (Variables|Default|SetbDestroyed true)
    (Game|Damage|ApplyRadialDamage 1.5e+02 (Math|Vector|MakeVector _x _y (+ _z 3e+01)) 5e+02 0 (Utilities|Array|MakeArray self) DamageCauser 0 true "ECC_Visibility")
    (CallFunction|PlayEffectsMulti)
    (Utilities|FlowControl|Delay 0.1)
    (Actor|DestroyActor)))

(fn ConstructionScript)