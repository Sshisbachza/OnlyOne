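; Projectile for the LSV Rhino's .50 cal gun that damages Rhinos and AH Sparrows on hit.
; On BeginPlay its collision ignores the instigator while moving.
; Hit checks for each vehicle class and applies that class's damage amount, naming the instigator as damage causer.
; All hits share a DoOnce that fires a radial impulse, spawns a machine-gun impact emitter and destroys the projectile after a brief delay.
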(event EventBeginPlay
  (Collision|IgnoreActorwhenMoving (Variables|MyProjectile|GetCollisionComponent) (Game|GetInstigator) true))

(event Collision|EventHit
  (params (MyComp :type Primitive%20Component%20Object%20Reference) (Other :type Actor%20Object%20Reference) (OtherComp :type Primitive%20Component%20Object%20Reference) (bSelfMoved :type Boolean) (HitLocation :type Vector) (HitNormal :type Vector :default "0, 0, 0") (NormalImpulse :type Vector :default "0, 0, 0") (Hit :type Hit%20Result%20Structure%20%28by%20ref%29))
  (bind _tracestart (Collision|BreakHitResult Hit))
  (bind (_x _y) (Math|Vector|BreakVector _tracestart))
  (Utilities|FlowControl|Sequence
    (:then_0
      ;[1 1 1] Damage caused to LSV_Rihno
      (if (== (Utilities|GetClass Other) "/Game/DVP/LSV-Rhino/Blueprints/BP_LSV_Rhino.BP_LSV_Rhino_C")
        (Game|Damage|ApplyDamage Other (Variables|Default|GetLSV_Rihno_damage_caused_to_LSV_Rihno) 0 (Game|GetInstigator))))
    (:then_1
      ;[1 1 1] Damage caused to AH_Sparrow
      (if (== (Utilities|GetClass Other) "/Game/DVP/AH-Sparrow/Blueprints/BP_AH_Sparrow.BP_AH_Sparrow_C")
        (Game|Damage|ApplyDamage Other (Variables|Default|GetLSV_Rihno_damage_caused_to_AH_Sparrow) 0 (Game|GetInstigator)))))
  (Utilities|FlowControl|DoOnce false
    (:Completed
      (Class|RadialForceComponent|FireImpulse (Variables|MyProjectile|GetRadialForce1))
      (Effects|SpawnEmitteratLocation "/Game/DVP/LSV-Rhino/Particles/PS_Impact_machine_gun.PS_Impact_machine_gun" HitLocation (Math|Rotator|MakeRotator _x _y 0.0))
      (Utilities|FlowControl|Delay 0.01)
      (Actor|DestroyActor))))

(fn ConstructionScript)