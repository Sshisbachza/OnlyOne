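; BP_AH_sparrow_Destroyed is the wreck actor for the destroyed AH Sparrow, handling its physical breakup, effects and cleanup.
; Once WreckDestroyed is true, Tick runs a one-time sequence that enables physics on all Body bones and applies radial force plus randomized tail and mast-rotor impulses.
; Explosion, fire and burning audio play for a delayed period, then a final explosion hides the mesh before the actor destroys itself.
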(event EventTick
  (params (DeltaSeconds :type Float%20%28single-precision%29))
  (bind _body (Variables|Default|GetBody))
  (bind _body_2 (Variables|Default|GetBody))
  (bind _body_3 (Variables|Default|GetBody))
  (bind _returnvalue (Transformation|GetWorldRotation _body_2))
  (if (Variables|Default|GetWreck_destroyed_?)
    (Utilities|FlowControl|DoOnce false
      (:Completed
        ;[1 1 1] Wake rigid bodes and add some force to them
        (Class|SkeletalMeshComponent|SetAllBodiesSimulatePhysics _body true)
        (Class|PrimitiveComponent|WakeAllRigidBodies _body)
        (Physics|AddRadialForce _body_2 (Transformation|GetActorLocation) 2.5e+02 (Math|Random|RandomFloatinRange 3e+04 1.5e+04) "RIF_Constant" true)
        (Physics|AddImpulse _body_3 (* (Math|Vector|GetRightVector _returnvalue) (Math|Random|RandomFloatinRange -2.5e+02 -3.5e+02)) "AH_Sparrow_Tail" true)
        (Class|PrimitiveComponent|AddAngularImpulse _body_3 (* (Math|Vector|GetUpVector _returnvalue) (Math|Random|RandomFloatinRange -15.0 15.0)) "AH_Sparrow__Mast_rotor" true)
        ;[1 1 1] Play primary PS effect, and play fire and explosion sound
        (Components|Activation|SetActive (Variables|Default|GetExplosion_1) true false)
        (Utilities|FlowControl|Delay 19.0) ; Change this to control how long PS effect will be played
        (Audio|Components|Audio|FadeOut (Variables|Default|GetFire_burning_Cue) 3.0 0.0 :!class /Script/Engine.AudioComponent)
        (Components|Activation|SetActive (Variables|Default|GetFire) false false)
        ;[1 1 1] Hide destroyed mesh, and play final PS effect
        (Utilities|FlowControl|Delay 2e+01) ; Change this to control how long destroyed mesh will be visible in game ( Be aware that particle life is allso calculated )
        (Components|Activation|SetActive (Variables|Default|GetExplosion_end) true false)
        (Rendering|SetVisibility (Variables|Default|GetBody) false false)
        (Utilities|FlowControl|Delay 2.0)
        (Actor|DestroyActor)))))

(fn ConstructionScript)