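; Projectile fired by the APC Puma's main gun, which ignores its instigator while moving.
; On hit it applies damage to the struck actor, then once fires a radial force impulse, spawns an impact particle effect and destroys itself after a brief delay.
; The impact effect's rotation is built from trace start coordinates rather than the surface normal.
; An unconnected class check is left available to restrict damage to Puma vehicles only.
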(event EventBeginPlay
  (Collision|IgnoreActorwhenMoving (Variables|MyProjectile|GetCollisionComponent) (Game|GetInstigator) true))

(event Collision|EventHit
  (params (MyComp :type Primitive%20Component%20Object%20Reference) (Other :type Actor%20Object%20Reference) (OtherComp :type Primitive%20Component%20Object%20Reference) (bSelfMoved :type Boolean) (HitLocation :type Vector) (HitNormal :type Vector :default "0, 0, 0") (NormalImpulse :type Vector :default "0, 0, 0") (Hit :type Hit%20Result%20Structure%20%28by%20ref%29))
  (bind _tracestart (Collision|BreakHitResult Hit))
  (bind (_x _y) (Math|Vector|BreakVector _tracestart))
  (Game|Damage|ApplyDamage Other (Variables|Default|GetAPC_Puma_damage_caused) 0 (Game|GetInstigator))
  (Utilities|FlowControl|DoOnce false
    (:Completed
      (Class|RadialForceComponent|FireImpulse (Variables|MyProjectile|GetRadialForce1))
      (Effects|SpawnEmitteratLocation "/Game/DVP/APC-Puma/Particles/PS_Impact_APC_main_gun.PS_Impact_APC_main_gun" HitLocation (Math|Rotator|MakeRotator _x _y 0.0))
      (Utilities|FlowControl|Delay 0.01)
      (Actor|DestroyActor))))

(fn ConstructionScript)